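; BP_LavaPool is a hazard that damages the player character at a set interval while it overlaps the pool.
; Begin overlap starts a looping timer, and end overlap clears it.
; ApplyEffects builds a GE_LavaPool spec on the player's ASC, passing negated LavaDamage through the Lava.Damage SetByCaller tag.
; It applies the spec to that ASC and adds each returned handle to the character's DamageEffects.
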(event `self.ReceiveActorBeginOverlap`
  (params (OtherActor :type "Actor Object Reference"))
  (if (== OtherActor (`GameplayStatics.GetPlayerCharacter` 0))
    (bind _returnvalue (`KismetSystemLibrary.K2_SetTimerDelegate` (`|CreateDelegate` :!event `Apply Effects`) (`self.LavaInterval`) true))
    (set `self.LavaEffectTimer` _returnvalue)))

(event `Apply Effects`
  (bind _asbp_top_down_character (cast `/Game/TopDown/Blueprints/BP_TopDownCharacter` (`GameplayStatics.GetPlayerCharacter` 0)))
  (bind _asc (`UTHUB_GAS2025Character.ASC` _asbp_top_down_character))
  (bind _returnvalue (`AbilitySystemBlueprintLibrary.AssignTagSetByCallerMagnitude` (`AbilitySystemComponent.MakeOutgoingSpec` :`self` _asc :`GameplayEffectClass` "/Game/GameplayEffects/Tarea2/GE_LavaPool.GE_LavaPool_C") (struct :`TagName` "Lava.Damage") (* (`self.LavaDamage`) -1.0)))
  (bind _returnvalue_2 (`AbilitySystemComponent.BP_ApplyGameplayEffectSpecToSelf` _asc _returnvalue))
  (`KismetArrayLibrary.Array_Add` (`/Game/TopDown/Blueprints/BP_TopDownCharacter.DamageEffects` _asbp_top_down_character) _returnvalue_2))

(event `self.ReceiveActorEndOverlap`
  (params (OtherActor :type "Actor Object Reference"))
  (if (== OtherActor (`GameplayStatics.GetPlayerCharacter` 0))
    (`KismetSystemLibrary.K2_ClearAndInvalidateTimerHandle` (`self.LavaEffectTimer`))))

(fn `UserConstructionScript`)