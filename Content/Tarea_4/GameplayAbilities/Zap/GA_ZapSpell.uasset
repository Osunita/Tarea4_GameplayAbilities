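; Gameplay ability for the Zap spell, which spawns BP_ZapSpell at the point under the mouse cursor.
; On activation it plays the attack montage, rotates the character using the cursor direction, disables movement and stores the cursor ray.
; The Spell.Zap gameplay event triggers a trace along that ray, spawns the spell, commits the cooldown and updates the HUD.
; Montage completion, blend-out or interruption ends the ability, restoring walking.
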(event `self.K2_ActivateAbility`
  (bind _returnvalue (`self.GetAvatarActorFromActorInfo`))
  (bind (_returnvalue_roll _returnvalue_pitch _returnvalue_yaw) (`KismetMathLibrary.BreakRotator` (`Actor.K2_GetActorRotation` _returnvalue)))
  (bind (_worldlocation _worlddirection) (`PlayerController.DeprojectMousePositionToWorld` (`GameplayStatics.GetPlayerController` 0)))
  (bind (_returnvalue_roll_2 _returnvalue_pitch_2 _returnvalue_yaw_2) (`KismetMathLibrary.BreakRotator` (`KismetMathLibrary.FindLookAtRotation` (`Actor.K2_GetActorLocation` _returnvalue) (`.ImpactPoint` (`GameplayStatics.BreakHitResult` (`PlayerController.GetHitResultUnderCursorByChannel` (`GameplayStatics.GetPlayerController` 0) "TraceTypeQuery1" true))))))
  (`AbilityTask_PlayMontageAndWait.CreatePlayMontageAndWaitProxy` "None" "/Game/Tarea_4/Anims/AM_SpellAttack.AM_SpellAttack" 1.5
    (:`then`
      (bind _asbp_top_down_character (cast `/Game/TopDown/Blueprints/BP_TopDownCharacter` (`self.GetAvatarActorFromActorInfo`)))
      (bind _output_get (set `self.As BP Top Down Character` _asbp_top_down_character))
      (`Actor.K2_SetActorRotation` _output_get (`KismetMathLibrary.RLerp` (`KismetMathLibrary.MakeRotator` 0.0 0.0 _returnvalue_yaw_2) (`KismetMathLibrary.MakeRotator` 0.0 0.0 _returnvalue_yaw)) true)
      (`CharacterMovementComponent.SetMovementMode` (`Character.CharacterMovement` _output_get) "MOVE_None" 0)
      (set `self.Start` _worldlocation)
      (set `self.End` (+ _worldlocation (* _worlddirection 1000000.0)))
      (`AbilityTask_WaitGameplayEvent.WaitGameplayEvent` (struct :`TagName` "Spell.Zap") null
        (:`EventReceived`
          (bind _outhit (`KismetSystemLibrary.LineTraceSingle` (`self.Start`) (`self.End`) "TraceTypeQuery1"))
          (`|SpawnActorFromClass` "/Game/Tarea_4/GameplayAbilities/Zap/BP_ZapSpell.BP_ZapSpell_C" (`KismetMathLibrary.MakeTransform` (`.Location` (`GameplayStatics.BreakHitResult` _outhit))) "Undefined" "MultiplyWithRoot" (`self.GetAvatarActorFromActorInfo`) null)
          (`self.K2_CommitAbilityCooldown` false true)
          (`self.RefreshUICooldown`))))
    (:`OnCompleted`
      (`self.K2_EndAbility` :!label _label))
    (:`OnBlendOut`
      (goto _label))
    (:`OnInterrupted`
      (goto _label))
    (:`OnCancelled`
      (goto _label))))

(event `self.K2_OnEndAbility`
  (params (bWasCancelled :type Boolean))
  (`KismetSystemLibrary.PrintString` "Zap")
  (`CharacterMovementComponent.SetMovementMode` (`Character.CharacterMovement` (`self.As BP Top Down Character`)) "MOVE_Walking" 0))

(event `RefreshUICooldown`
  ;[1 1 1] UI Cooldown
  (`/Game/TopDown/Blueprints/BP_HUDTopDown.SetCooldowns` (`/Game/TopDown/Blueprints/BP_TopDownPlayerController.GetHudRef` (`/Game/TopDown/Blueprints/BP_TopDownCharacter.GetPCRef` (`self.As BP Top Down Character`))) (`self.GetCooldownTimeRemaining`)))