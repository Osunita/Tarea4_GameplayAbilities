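; Zap spell actor that deals one-shot damage through the Gameplay Ability System where it spawns.
; On BeginPlay it plays a non-spatial zap sound and runs a single box trace for Pawns at its own location, with debug drawing left on.
; If the hit actor has an AbilitySystemComponent, the spell owner's ASC applies GE_ContactDamage to it.
; The owner's ASC is used without a validity check.
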(event `self.ReceiveBeginPlay`
  (bind _returnvalue (`self.K2_GetActorLocation`))
  (bind _returnvalue_2 (`AbilitySystemBlueprintLibrary.GetAbilitySystemComponent` (`self.GetOwner`)))
  (`GameplayStatics.PlaySound2D` "/Game/Zap_VFX/Audio/SFX_Vefects_Zap_Medium_02_Cue.SFX_Vefects_Zap_Medium_02_Cue" 1.5 1.0 0.0 null null)
  (bind _outhit (`KismetSystemLibrary.BoxTraceSingleForObjects` :`Start` _returnvalue :`End` _returnvalue :`HalfSize` (48.0 48.0 48.0) :`ObjectTypes` (`|MakeArray` "ObjectTypeQuery3" :!type "EObjectTypeQuery Enum") :`DrawDebugType` "ForDuration"))
  (bind _returnvalue_3 (`self.GetComponentByClass` (`.HitActor` (`GameplayStatics.BreakHitResult` _outhit)) "/Script/GameplayAbilities.AbilitySystemComponent"))
  (if (and (`GameplayStatics.BreakHitResult` _outhit) (`KismetSystemLibrary.IsValid` _returnvalue_3))
    (`AbilitySystemComponent.BP_ApplyGameplayEffectSpecToTarget` _returnvalue_2 (`AbilitySystemComponent.MakeOutgoingSpec` _returnvalue_2 "/Game/GameplayEffects/Tarea2/GE_ContactDamage.GE_ContactDamage_C" 0.0 (`AbilitySystemComponent.MakeEffectContext` _returnvalue_2)) _returnvalue_3)))

(fn `UserConstructionScript`)