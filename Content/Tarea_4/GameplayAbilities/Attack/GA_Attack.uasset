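; Melee attack gameplay ability for the top-down character that plays the attack montage facing the point under the cursor.
; Movement is disabled during the attack and restored to walking when the ability ends.
; The Attack.Attack gameplay event triggers a debug-drawn box trace at the right hand for pawns.
; A hit on a target with an ability system component applies GE_ContactDamage and commits the cooldown, so misses incur none.
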(event `self.K2_ActivateAbility`
  (bind _returnvalue (`self.GetAvatarActorFromActorInfo`))
  (bind _returnvalue_2 (`self.GetAbilitySystemComponentFromActorInfo`))
  (bind _returnvalue_3 (`self.GetAvatarActorFromActorInfo`))
  (bind (_returnvalue_roll _returnvalue_pitch _returnvalue_yaw) (`KismetMathLibrary.BreakRotator` (`Actor.K2_GetActorRotation` _returnvalue_3)))
  (bind _returnvalue_4 (`SceneComponent.GetSocketLocation` (`Actor.GetComponentByClass` _returnvalue "/Script/Engine.SkeletalMeshComponent") "hand_r"))
  (bind (_returnvalue_roll_2 _returnvalue_pitch_2 _returnvalue_yaw_2) (`KismetMathLibrary.BreakRotator` (`KismetMathLibrary.FindLookAtRotation` (`Actor.K2_GetActorLocation` _returnvalue_3) (`.ImpactPoint` (`GameplayStatics.BreakHitResult` (`PlayerController.GetHitResultUnderCursorByChannel` (`GameplayStatics.GetPlayerController` 0) "TraceTypeQuery1" true))))))
  (`AbilityTask_PlayMontageAndWait.CreatePlayMontageAndWaitProxy` "None" "/Game/Tarea_4/Anims/AM_Attack.AM_Attack" 1.5
    (:`then`
      (bind _asbp_top_down_character (cast `/Game/TopDown/Blueprints/BP_TopDownCharacter` (`self.GetAvatarActorFromActorInfo`)))
      (bind _output_get (set `self.As BP Top Down Character` _asbp_top_down_character))
      (`Actor.K2_SetActorRotation` _output_get (`KismetMathLibrary.RLerp` (`KismetMathLibrary.MakeRotator` 0.0 0.0 _returnvalue_yaw_2) (`KismetMathLibrary.MakeRotator` 0.0 0.0 _returnvalue_yaw)) true)
      (`CharacterMovementComponent.SetMovementMode` (`Character.CharacterMovement` _output_get) "MOVE_None" 0)
      (`AbilityTask_WaitGameplayEvent.WaitGameplayEvent` (struct :`TagName` "Attack.Attack") null
        (:`EventReceived`
          (bind _outhit (`KismetSystemLibrary.BoxTraceSingleForObjects` _returnvalue_4 _returnvalue_4 (48.0 64.0 32.0) (`Actor.K2_GetActorRotation` _returnvalue) (`|MakeArray` "ObjectTypeQuery3" :!type "EObjectTypeQuery Enum") false (`|MakeArray` (`self.GetAvatarActorFromActorInfo`)) "ForDuration"))
          (bind _returnvalue_5 (`Actor.GetComponentByClass` (`.HitActor` (`GameplayStatics.BreakHitResult` _outhit)) "/Script/GameplayAbilities.AbilitySystemComponent"))
          (if (and (`GameplayStatics.BreakHitResult` _outhit) (`KismetSystemLibrary.IsValid` _returnvalue_5))
            (`AbilitySystemComponent.BP_ApplyGameplayEffectSpecToTarget` _returnvalue_2 (`AbilitySystemComponent.MakeOutgoingSpec` _returnvalue_2 "/Game/GameplayEffects/Tarea2/GE_ContactDamage.GE_ContactDamage_C" 0.0 (`AbilitySystemComponent.MakeEffectContext` _returnvalue_2)) _returnvalue_5)
            (`self.K2_CommitAbilityCooldown` false true)))))
    (:`OnCompleted`
      (`self.K2_EndAbility` :!label _label))
    (:`OnBlendOut`
      (goto _label))
    (:`OnInterrupted`
      (goto _label))
    (:`OnCancelled`
      (goto _label))))

(event `self.K2_OnEndAbility`
  (params (bWasCancelled :type Boolean))
  (`CharacterMovementComponent.SetMovementMode` (`Character.CharacterMovement` (`self.As BP Top Down Character`)) "MOVE_Walking" 0))